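; MasterAI_BP is an AI character with a named health bar widget, shown while the player overlaps its sphere.
; DoSomeDamage makes head hits play a sound and trigger a delayed random move before resuming controller AIMovement, without reducing health.
; Other hits subtract StunDamage; at zero health it simulates physics, disables capsule collision, hides the bar and is destroyed after a delay.
; TalktoPlayer increments an index and prints that dialogue line.
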(event `self.ReceiveBeginPlay`
  (set `self.CurrentHealth` (`self.MaxHealth`))
  (bind _asaihealthhbar (cast `/Game/Blueprints/UI/AIHealthhbar` (`WidgetComponent.GetUserWidgetObject` (`self.AIhealthbar`))))
  (bind _output_get (set `self.AIHealthhbarREF` _asaihealthhbar))
  (set `/Game/Blueprints/UI/AIHealthhbar.Owner` self _output_get)
  ;[1 1 1] Get AI Name
  (`TextBlock.SetText` (`/Game/Blueprints/UI/AIHealthhbar.AI_Name` (`self.AIHealthhbarREF`)) (`KismetTextLibrary.Conv_StringToText` (`self.Name`))))

(event `self.Sphere.OnComponentBeginOverlap`
  (params (OverlappedComponent :type "PrimitiveComponent Object Reference") (OtherActor :type "Actor Object Reference") (OtherComp :type "PrimitiveComponent Object Reference") (OtherBodyIndex :type Integer) (bFromSweep :type Boolean) (SweepResult :type "HitResult Structure (by ref)"))
  (cast `/Game/Blueprints/PlayerLogic/NineTo5_Character` OtherActor)
  (`SceneComponent.SetVisibility` (`self.AIhealthbar`) true false))

(event `self.Sphere.OnComponentEndOverlap`
  (params (OverlappedComponent :type "PrimitiveComponent Object Reference") (OtherActor :type "Actor Object Reference") (OtherComp :type "PrimitiveComponent Object Reference") (OtherBodyIndex :type Integer))
  (cast `/Game/Blueprints/PlayerLogic/NineTo5_Character` OtherActor)
  (`SceneComponent.SetVisibility` (`self.AIhealthbar`) false false))

(event `/Game/Blueprints/PlayerLogic/DoSomeDamage_BPI.DoSomeDamage`
  (params (BoneName :type Name) (StunDamage :type "Float (double-precision)"))
  ;[1 1 1] AI Health system
  (if (== BoneName "head")
    (`GameplayStatics.PlaySound2D` "/Game/Blueprints/PlayerLogic/Sounds/Oneliners/Bellend_Cue.Bellend_Cue" 1.0 1.0 0.0 null null)
    (`KismetSystemLibrary.Delay` 2.0)
    (`|AIMoveTo` null (`NavigationSystemV1.K2_GetRandomReachablePointInRadius` (`self.K2_GetActorLocation`) 500.0 null "/Script/AIModule.NavFilter_AIControllerDefault") null
      (:`OnSuccess`
        (`/Game/Blueprints/AI/AI_Logic/AI_MasterController.AI_Movement` (cast `/Game/Blueprints/AI/AI_Logic/AI_MasterController` (`AIBlueprintHelperLibrary.GetAIController` null) :!pure true))))
    (else
      (bind _output_get (set `self.CurrentHealth` (- (`self.CurrentHealth`) StunDamage)))
      (if (<= _output_get 0.0)
        (`/Engine/EditorBlueprintResources/StandardMacros.DoOnce` false
          (:`Completed`
            (set `self.AI_IsDead` true)
            (`SkeletalMeshComponent.SetAllBodiesSimulatePhysics` (`self.Mesh`) true)
            (`PrimitiveComponent.SetCollisionEnabled` (`self.CapsuleComponent`) "NoCollision")
            (`SceneComponent.SetVisibility` (`self.AIhealthbar`) false false)
            (`KismetSystemLibrary.Delay` 10.0)
            (`self.K2_DestroyActor`)))))))

(event `/Game/Blueprints/AI/AI_Logic/BPI_Dialogue.TalkToPlayer`
  (`/Engine/EditorBlueprintResources/StandardMacros.IncrementInt` (`self.DialogueIndex`)
    (:`  `
      (`KismetSystemLibrary.PrintString` (`|GetArrayItem` (`self.Dialogue`) (`self.DialogueIndex`))))))

(fn `UserConstructionScript`)