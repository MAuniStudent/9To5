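; Game instance for 9to5 that owns the game's save object and handles loading and saving it to a slot.
; On Init it synchronously loads the slot, or creates a fresh 9to5Save if none exists, and caches it for GetGameData.
; Load and save each offer sync or async paths, but only a completed async load calls OnGameLoaded.
; SavePlayer writes player data into the cached object and then saves it.
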(event `self.ReceiveInit`
  (`self.LoadGameData` false))

(event `/Game/Blueprints/PlayerLogic/SavedData/BPI_SavGameData.LoadGameData`
  (params (Async :type Boolean))
  (bind _returnvalue (`GameplayStatics.DoesSaveGameExist` (`self.SaveSlotName`)))
  (if _returnvalue
    (if Async
      (bind _savegame (`AsyncActionHandleSaveGame.AsyncLoadGameFromSlot` (`self.SaveSlotName`))
        (:`Completed`
          (bind _as9to_5save (cast `/Game/Blueprints/PlayerLogic/SavedData/9to5Save` _savegame))
          (set `self.SAVEDataREF` _as9to_5save)
          (`self.OnGameLoaded`)))
      (else
        (bind _returnvalue_2 (`GameplayStatics.LoadGameFromSlot` (`self.SaveSlotName`)))
        (bind _as9to_5save_2 (cast `/Game/Blueprints/PlayerLogic/SavedData/9to5Save` _returnvalue_2))
        (set `self.SAVEDataREF` _as9to_5save_2)))
    (else
      (bind _returnvalue_3 (`GameplayStatics.CreateSaveGameObject` "/Game/Blueprints/PlayerLogic/SavedData/9to5Save.9to5Save_C"))
      (set `self.SAVEDataREF` _returnvalue_3))))

(event `/Game/Blueprints/PlayerLogic/SavedData/BPI_SavGameData.SaveGameData`
  (params (Async :type Boolean))
  (if Async
    (`AsyncActionHandleSaveGame.AsyncSaveGameToSlot` (`self.SAVEDataREF`) (`self.SaveSlotName`))
    (else
      (`GameplayStatics.SaveGameToSlot` (`self.SAVEDataREF`) (`self.SaveSlotName`)))))

(event `/Game/Blueprints/PlayerLogic/SavedData/BPI_SavGameData.SavePlayer`
  (params (PlayerData :type "/Game/Blueprints/PlayerLogic/SavedData/S_PlayerSaves Structure") (Async :type Boolean))
  (set `/Game/Blueprints/PlayerLogic/SavedData/9to5Save.PlayerSaves` PlayerData (`self.SAVEDataREF`))
  (`self.SaveGameData` Async))

(fn `GetGameData`
  (returns (SavedData :type "/Game/Blueprints/PlayerLogic/SavedData/9to5Save Object Reference"))
  (return (`self.SAVEDataREF`)))