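; Base weapon actor that the NineTo5 character can pick up in the world.
; Sphere overlap toggles the pickup widget and pick-up flag, filling in icon and name from WeaponInfo and enabling input on entry.
; Interact passes the weapon to the character's WeaponPickup, while ClearPickupGarbage hides widget and Niagara effect and destroys the sphere.
; The construction script writes the actor's own class into the WeaponInfo struct, keeping its other fields.
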(event `self.Sphere.OnComponentBeginOverlap`
  (params (OverlappedComponent :type "PrimitiveComponent Object Reference") (OtherActor :type "Actor Object Reference") (OtherComp :type "PrimitiveComponent Object Reference") (OtherBodyIndex :type Integer) (bFromSweep :type Boolean) (SweepResult :type "HitResult Structure (by ref)"))
  (bind ((`Image_8_406D9029421CFF013FF8B1B1123D2BD1` _image) (`Name_11_674A8D344EA60AAEF058C0B860BE2528` _name)) (break `/Game/Blueprints/Weapons/S_WeaponInfo` (`self.WeaponInfo`)))
  (bind _asweapon_pickup_wb (cast `/Game/Blueprints/UI/WeaponPickup_WB` (`WidgetComponent.GetUserWidgetObject` (`self.Widget`)) :!pure true))
  (bind _asnine_to_5_character (cast `/Game/Blueprints/PlayerLogic/NineTo5_Character` OtherActor))
  (set `self.NineTo5CharacterREF` _asnine_to_5_character)
  (`SceneComponent.SetVisibility` (`self.Widget`) true false)
  (set `self.CanPick?` true)
  (`self.EnableInput` (`GameplayStatics.GetPlayerController` 0))
  ;[0.3594 0.1781 0] Set the appropriate weapon icon and weapon name dynamicaly
  (set `/Game/Blueprints/UI/WeaponPickup_WB.WeaponIcon` _image _asweapon_pickup_wb)
  (set `/Game/Blueprints/UI/WeaponPickup_WB.WeaponName` (`KismetTextLibrary.Conv_StringToText` _name) _asweapon_pickup_wb))

(event `self.Sphere.OnComponentEndOverlap`
  (params (OverlappedComponent :type "PrimitiveComponent Object Reference") (OtherActor :type "Actor Object Reference") (OtherComp :type "PrimitiveComponent Object Reference") (OtherBodyIndex :type Integer))
  (bind _asnine_to_5_character (cast `/Game/Blueprints/PlayerLogic/NineTo5_Character` OtherActor))
  (set `self.NineTo5CharacterREF` _asnine_to_5_character)
  (`SceneComponent.SetVisibility` (`self.Widget`) false false)
  (set `self.CanPick?` false))

(event `EnhancedInput|/Game/Blueprints/Input/Actions/IA_Interact`
  (params (ActionValue :type Boolean) (ElapsedSeconds :type "Float (double-precision)") (TriggeredSeconds :type "Float (double-precision)") (InputAction :type "InputAction Object Reference" :default "/Game/Blueprints/Input/Actions/IA_Interact.IA_Interact"))
  (:`Started`
    (if (`self.CanPick?`)
      ;[0 0.505 1] Weapon Pickup is set to self, all variables for weapon are in the construction script
      (`/Game/Blueprints/PlayerLogic/NineTo5_Character.WeaponPickup` (`self.NineTo5CharacterREF`) self))))

(event `ClearPickupGarbage`
  ;[1 0 0] function to disable VFX and UI and overlap sphere
  (`SceneComponent.SetVisibility` (`self.Widget`) false false)
  (`SceneComponent.SetVisibility` (`self.Niagara`) false false)
  (`ActorComponent.K2_DestroyComponent` (`self.Sphere`)))

(fn `UserConstructionScript`
  (bind (_weaponinfo_weapontype _weaponinfo_class _weaponinfo_image _weaponinfo_name _weaponinfo_damage _weaponinfo_range _weaponinfo_firerate _weaponinfo_clipsize _weaponinfo_ammo _weaponinfo_maxammo _weaponinfo_ammopickup _weaponinfo_equipsocket _weaponinfo_unequipsocket _weaponinfo_equipmontage _weaponinfo_unequipmontage _weaponinfo_pickupmontage _weaponinfo_reloadmontage _weaponinfo_fireweaponmontage _weaponinfo_weaponsound) (break `/Game/Blueprints/Weapons/S_WeaponInfo` (`self.WeaponInfo`)))
  (set `self.WeaponInfo` (make `/Game/Blueprints/Weapons/S_WeaponInfo` _weaponinfo_weapontype (`GameplayStatics.GetObjectClass` self) _weaponinfo_image _weaponinfo_name _weaponinfo_damage _weaponinfo_range _weaponinfo_firerate _weaponinfo_clipsize _weaponinfo_ammo _weaponinfo_maxammo _weaponinfo_ammopickup _weaponinfo_equipsocket _weaponinfo_unequipsocket _weaponinfo_equipmontage _weaponinfo_unequipmontage _weaponinfo_pickupmontage _weaponinfo_reloadmontage _weaponinfo_fireweaponmontage _weaponinfo_weaponsound)))