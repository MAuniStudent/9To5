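; Nerf ammo pickup that refills the current weapon when a NineTo5_Character with the Nerf equipped overlaps its sphere.
; If MaxAmmo already equals PickupAmmo it prints "Ammo full" and stays.
; Otherwise it writes the weapon's MaxAmmo, plays a sound, spawns a particle burst and destroys itself.
; The cap check compares the sum against PickupAmmo, so any non-negative MaxAmmo is set to PickupAmmo, not added to.
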(event `self.Sphere.OnComponentBeginOverlap`
  (params (OverlappedComponent :type "PrimitiveComponent Object Reference") (OtherActor :type "Actor Object Reference") (OtherComp :type "PrimitiveComponent Object Reference") (OtherBodyIndex :type Integer) (bFromSweep :type Boolean) (SweepResult :type "HitResult Structure (by ref)"))
  (bind _asnine_to_5_character (cast `/Game/Blueprints/PlayerLogic/NineTo5_Character` OtherActor))
  (bind _output_get (set `self.NineTo5REF` _asnine_to_5_character))
  (if (`/Game/Blueprints/PlayerLogic/NineTo5_Character.EquipNerf` _output_get)
    (`self.AddAmmo`)))

(event `AddAmmo`
  (bind _weaponinfo (`/Game/Blueprints/Weapons/WeaponMaster_BP.WeaponInfo` (`/Game/Blueprints/PlayerLogic/NineTo5_Character.CurrentWeaponBP` (`self.NineTo5REF`))))
  (bind ((`MaxAmmo_21_5327668A477219D80E419580CE0BBF41` _maxammo)) (break `/Game/Blueprints/Weapons/S_WeaponInfo` (`/Game/Blueprints/Weapons/WeaponMaster_BP.WeaponInfo` (`/Game/Blueprints/PlayerLogic/NineTo5_Character.CurrentWeaponBP` (`self.NineTo5REF`)))))
  (bind _returnvalue (+ (`self.PickupAmmo`) _maxammo))
  (if (== _maxammo (`self.PickupAmmo`))
    (`KismetSystemLibrary.PrintString` "Ammo full")
    (else
      (if (>= _returnvalue (`self.PickupAmmo`))
        (setmembers `/Game/Blueprints/Weapons/S_WeaponInfo` :`StructRef` _weaponinfo :`MaxAmmo` (`self.PickupAmmo`))
        (else
          (setmembers `/Game/Blueprints/Weapons/S_WeaponInfo` :`StructRef` _weaponinfo :`MaxAmmo` _returnvalue)))
      (`GameplayStatics.PlaySound2D` "/Game/Blueprints/PlayerLogic/Sounds/Oneliners/Nice.Nice" 1.0 1.0 0.0 null null)
      (`GameplayStatics.SpawnEmitterAtLocation` "/Game/Blueprints/VFX/Realistic_Starter_VFX_Pack_Vol2/Particles/Destruction/P_Destruction_Glass.P_Destruction_Glass" (`self.K2_GetActorLocation`))
      (`self.K2_DestroyActor` self))))

(fn `UserConstructionScript`)