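; Stealth locker the player character can hide in, with input enabled and gated by overlap with its trigger box.
; The hide action toggles the character's visibility and collision and blends the view between locker and player.
; Each use plays a slam sound and a delayed door-swing timeline, while the first also plays heavy breathing and a timed speech-bubble widget sequence.
; AI controller code in the hiding function is disconnected.
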(event `EnhancedInput|/Game/Blueprints/Input/Actions/IA_HideAway`
  (params (ActionValue :type Boolean) (ElapsedSeconds :type "Float (double-precision)") (TriggeredSeconds :type "Float (double-precision)") (InputAction :type "InputAction Object Reference" :default "/Game/Blueprints/Input/Actions/IA_HideAway.IA_HideAway"))
  ;[1 1 1] Use locker for stealth to hide in
  (:`Started`
    (`/Engine/EditorBlueprintResources/StandardMacros.Gate` true :!label _label
      (:`Exit`
        (`|ExecutionSequence`
          (:`then_0`
            (`self.HidingON/OFF`)
            (`KismetSystemLibrary.Delay` 0.2)
            (`self.EnableInput` self (`GameplayStatics.GetPlayerController` 0) :!label _label_2)
            (goto _label :!via `Open`))
          (:`then_1`
            (`|ExecutionSequence`
              (:`then_0`
                (`KismetSystemLibrary.Delay` 1.0)
                (bind (_direction _door) (`Timeline|UseLockerDoor` :!via `PlayFromStart`)
                  (:`Update`
                    (`SceneComponent.K2_SetRelativeRotation` (`self.LockerDoor`) (`KismetMathLibrary.MakeRotator` 0.0 0.0 (`KismetMathLibrary.Lerp` (`self.ClosedDoorAngle`) (`self.OpenDoorAngle`) _door)) false false)
                    (`/Engine/EditorBlueprintResources/StandardMacros.DoOnce` false
                      (:`Completed`
                        (`GameplayStatics.PlaySound2D` "/Game/Blueprints/Sounds/heavy-breathing.heavy-breathing" 1.0 1.0 0.0 null null)
                        (`KismetSystemLibrary.Delay` 4.0)
                        (bind _returnvalue (`|CreateWidget` "/Game/Blueprints/UI/Stealth_WB.Stealth_WB_C" (`GameplayStatics.GetPlayerController` 0)))
                        (bind _output_get (set `self.StealthREF` _returnvalue))
                        (`UserWidget.AddToViewport` _output_get 0)
                        (`Widget.SetVisibility` (`/Game/Blueprints/UI/Stealth_WB.LeftBubble` (`self.StealthREF`)) "Visible")
                        (`Widget.SetVisibility` (`/Game/Blueprints/UI/Stealth_WB.Skive` (`self.StealthREF`)) "Visible")
                        (`KismetSystemLibrary.Delay` 3.0)
                        (`Widget.SetVisibility` (`/Game/Blueprints/UI/Stealth_WB.RightBubble` (`self.StealthREF`)) "Visible")
                        (`Widget.SetVisibility` (`/Game/Blueprints/UI/Stealth_WB.Home` (`self.StealthREF`)) "Visible")
                        (`KismetSystemLibrary.Delay` 2.0)
                        (`Widget.SetVisibility` (`/Game/Blueprints/UI/Stealth_WB.Gone` (`self.StealthREF`)) "Visible")
                        (`KismetSystemLibrary.Delay` 4.0)
                        (`Widget.RemoveFromParent` (`self.StealthREF`)))))))
              (:`then_1`
                (`GameplayStatics.PlaySound2D` "/Game/Blueprints/Interaction/StealthLocker/sound/lockerdoor-slamming.lockerdoor-slamming" 1.0 1.0 0.0 null null)))))))))

(event `self.Box.OnComponentBeginOverlap`
  (params (OverlappedComponent :type "PrimitiveComponent Object Reference") (OtherActor :type "Actor Object Reference") (OtherComp :type "PrimitiveComponent Object Reference") (OtherBodyIndex :type Integer) (bFromSweep :type Boolean) (SweepResult :type "HitResult Structure (by ref)"))
  ;[1 1 1] Use locker for stealth to hide in
  (bind _asnine_to_5_character (cast `/Game/Blueprints/PlayerLogic/NineTo5_Character` OtherActor))
  (set `self.NineTo5_REF` _asnine_to_5_character)
  (goto _label_2))

(event `self.Box.OnComponentEndOverlap`
  (params (OverlappedComponent :type "PrimitiveComponent Object Reference") (OtherActor :type "Actor Object Reference") (OtherComp :type "PrimitiveComponent Object Reference") (OtherBodyIndex :type Integer))
  ;[1 1 1] Use locker for stealth to hide in
  (bind _asnine_to_5_character (cast `/Game/Blueprints/PlayerLogic/NineTo5_Character` OtherActor))
  (set `self.NineTo5_REF` _asnine_to_5_character)
  (`self.DisableInput` self (`GameplayStatics.GetPlayerController` 0))
  (goto _label :!via `Close`))

(event `EnhancedInput|/Game/Blueprints/Input/Actions/IA_Look`
  (params (ActionValue :type "Vector2D Structure") (ElapsedSeconds :type "Float (double-precision)") (TriggeredSeconds :type "Float (double-precision)") (InputAction :type "InputAction Object Reference" :default "/Game/Blueprints/Input/Actions/IA_Look.IA_Look")))

(fn `HidingON/OFF`
  (bind _returnvalue (`GameplayStatics.GetPlayerController` 0))
  (bind _nineto5_ref (`self.NineTo5_REF`))
  (if (`self.IsHiding?`)
    (set `self.IsHiding?` false)
    (`self.SetActorHiddenInGame` _nineto5_ref false)
    (`self.SetActorEnableCollision` _nineto5_ref true)
    (`PlayerController.SetViewTargetWithBlend` _returnvalue _nineto5_ref 1.0 "VTBlend_Linear" 0.0 false)
    (else
      (set `self.IsHiding?` true)
      (`self.SetActorHiddenInGame` _nineto5_ref true)
      (`self.SetActorEnableCollision` _nineto5_ref false)
      (`PlayerController.SetViewTargetWithBlend` _returnvalue self 1.0 "VTBlend_Linear" 0.0 false))))

(fn `UserConstructionScript`)