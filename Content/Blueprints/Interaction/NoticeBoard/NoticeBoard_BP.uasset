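; Notice board actor that gives a NineTo5_Character a zoomed view while it stands inside the board's Box trigger.
; On begin overlap it swaps the character's FollowCamera for its ZoomCam, and on end overlap it swaps them back.
; A DoOnce sets the character's IsHackable flag on the first entry only, and leaving does not clear it.
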(event `self.Box.OnComponentBeginOverlap`
  (params (OverlappedComponent :type "PrimitiveComponent Object Reference") (OtherActor :type "Actor Object Reference") (OtherComp :type "PrimitiveComponent Object Reference") (OtherBodyIndex :type Integer) (bFromSweep :type Boolean) (SweepResult :type "HitResult Structure (by ref)"))
  (bind _asnine_to_5_character (cast `/Game/Blueprints/PlayerLogic/NineTo5_Character` OtherActor))
  (`ActorComponent.SetActive` (`/Game/Blueprints/PlayerLogic/NineTo5_Character.FollowCamera` _asnine_to_5_character) false false)
  (`ActorComponent.SetActive` (`/Game/Blueprints/PlayerLogic/NineTo5_Character.ZoomCam` _asnine_to_5_character) true false)
  (`/Engine/EditorBlueprintResources/StandardMacros.DoOnce` false
    (:`Completed`
      (set `/Game/Blueprints/PlayerLogic/NineTo5_Character.IsHackable` true _asnine_to_5_character))))

(event `self.Box.OnComponentEndOverlap`
  (params (OverlappedComponent :type "PrimitiveComponent Object Reference") (OtherActor :type "Actor Object Reference") (OtherComp :type "PrimitiveComponent Object Reference") (OtherBodyIndex :type Integer))
  (bind _asnine_to_5_character (cast `/Game/Blueprints/PlayerLogic/NineTo5_Character` OtherActor))
  (`ActorComponent.SetActive` (`/Game/Blueprints/PlayerLogic/NineTo5_Character.ZoomCam` _asnine_to_5_character) false false)
  (`ActorComponent.SetActive` (`/Game/Blueprints/PlayerLogic/NineTo5_Character.FollowCamera` _asnine_to_5_character) true false))

(fn `UserConstructionScript`)